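; Game instance that owns the game's UI screens and the flow between the main menu, gameplay and pause.
; Show events lazily create and cache each widget, then add it to the viewport; the pistol pickup widget removes itself after one second.
; Start and pause events switch input mode and cursor, with pausing also freezing the game.
; New game and confirmed return to menu show a loading screen, then async-load the map.
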(event `Show Start Game`
  (bind _returnvalue (`GameplayStatics.GetPlayerController` 0))
  (`/Engine/EditorBlueprintResources/StandardMacros.IsValid` (`self.StartGameWB`)
    (:`Is Valid`
      _)
    (:`Is Not Valid`
      (bind _returnvalue_2 (`|CreateWidget` "/Game/UI/Menu/StartGameWB.StartGameWB_C" _returnvalue))
      (set `self.StartGameWB` _returnvalue_2)))
  (`UserWidget.AddToViewport` (`self.StartGameWB`) 0)
  (set `PlayerController.bShowMouseCursor` true _returnvalue)
  (`WidgetBlueprintLibrary.SetInputMode_UIOnlyEx` _returnvalue (`self.StartGameWB`) "LockInFullscreen"))

(event `Show Main Menu`
  (`/Engine/EditorBlueprintResources/StandardMacros.IsValid` (`self.MainMenuWB`)
    (:`Is Valid`
      _)
    (:`Is Not Valid`
      (bind _returnvalue (`|CreateWidget` "/Game/UI/Menu/MainMenuWB.MainMenuWB_C" (`GameplayStatics.GetPlayerController` 0)))
      (set `self.MainMenuWB` _returnvalue)))
  (`UserWidget.AddToViewport` (`self.MainMenuWB`) 0))

(event `Show Loading Screen`
  (`/Engine/EditorBlueprintResources/StandardMacros.IsValid` (`self.LoadingScreenWB`)
    (:`Is Valid`
      _)
    (:`Is Not Valid`
      (bind _returnvalue (`|CreateWidget` "/Game/UI/Menu/LoadingScreenWB.LoadingScreenWB_C" (`GameplayStatics.GetPlayerController` 0)))
      (set `self.LoadingScreenWB` _returnvalue)))
  (`UserWidget.AddToViewport` (`self.LoadingScreenWB`) 0))

(event `ShowSettingsMenu`
  (`/Engine/EditorBlueprintResources/StandardMacros.IsValid` (`self.SettingsMenuWB`)
    (:`Is Valid`
      _)
    (:`Is Not Valid`
      (bind _returnvalue (`|CreateWidget` "/Game/UI/Menu/SettingsMenuWB.SettingsMenuWB_C" (`GameplayStatics.GetPlayerController` 0)))
      (set `self.SettingsMenuWB` _returnvalue)))
  (`UserWidget.AddToViewport` (`self.SettingsMenuWB`) 0))

(event `ShowPickedItem`
  (`/Engine/EditorBlueprintResources/StandardMacros.IsValid` (`self.PistolWB`)
    (:`Is Valid`
      _)
    (:`Is Not Valid`
      (bind _returnvalue (`|CreateWidget` "/Game/UI/Inventory/PistolWB.PistolWB_C" (`GameplayStatics.GetPlayerController` 0)))
      (set `self.PistolWB` _returnvalue)))
  (`UserWidget.AddToViewport` (`self.PistolWB`) 0)
  (`KismetSystemLibrary.Delay` 1.0)
  (`Widget.RemoveFromParent` (`self.PistolWB`)))

(event `Create New Game`
  (set `PlayerController.bShowMouseCursor` false (`GameplayStatics.GetPlayerController` 0))
  (`WidgetBlueprintLibrary.SetInputMode_GameOnly` (`GameplayStatics.GetPlayerController` 0))
  (`self.Show Loading Screen`)
  (`KismetSystemLibrary.Delay` 1.0)
  (`self.AsyncLevelLoad` "/Game/Maps/" "ThirdPersonMap"))

(event `Show Pause Menu`
  (bind _returnvalue (`GameplayStatics.GetPlayerController` 0))
  (`/Engine/EditorBlueprintResources/StandardMacros.IsValid` (`self.PauseMenuWB`)
    (:`Is Valid`
      _)
    (:`Is Not Valid`
      (bind _returnvalue_2 (`|CreateWidget` "/Game/UI/Menu/PauseMenuWB.PauseMenuWB_C" _returnvalue))
      (set `self.PauseMenuWB` _returnvalue_2)))
  (`UserWidget.AddToViewport` (`self.PauseMenuWB`) 0)
  (`WidgetBlueprintLibrary.SetInputMode_UIOnlyEx` _returnvalue (`self.PauseMenuWB`) "LockInFullscreen")
  (`GameplayStatics.SetGamePaused` true)
  (set `PlayerController.bShowMouseCursor` true _returnvalue))

(event `Pause Menu: Resume`
  (bind _returnvalue (`GameplayStatics.GetPlayerController` 0))
  (`Widget.RemoveFromParent` (`self.PauseMenuWB`))
  (`GameplayStatics.SetGamePaused` false)
  (`WidgetBlueprintLibrary.SetInputMode_GameOnly` _returnvalue)
  (set `PlayerController.bShowMouseCursor` false _returnvalue))

(event `Pause Menu: Go To Main Menu`
  (`/Engine/EditorBlueprintResources/StandardMacros.IsValid` (`self.PauseMenuToMainMenuWB`)
    (:`Is Valid`
      _)
    (:`Is Not Valid`
      (bind _returnvalue (`|CreateWidget` "/Game/UI/Menu/PauseToMainMenuWB.PauseToMainMenuWB_C" (`GameplayStatics.GetPlayerController` 0)))
      (set `self.PauseMenuToMainMenuWB` _returnvalue)))
  (`UserWidget.AddToViewport` (`self.PauseMenuToMainMenuWB`) 0))

(event `Pause Menu: Go To Main Menu: accept`
  (`self.Show Loading Screen`)
  (`self.AsyncLevelLoad` "/Game/Maps/" "MainMenu"))

(event `Pause Menu: Go To Main Menu: decline`
  (`Widget.RemoveFromParent` (`self.PauseMenuToMainMenuWB`)))