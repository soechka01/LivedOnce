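; MainWeapon is a pickup-capable weapon actor that hands itself to the interactor's WeaponSystemComponent when interacted with.
; An overlap area shows a lazily created prompt widget with the weapon name and sets CanPick while the player character is inside.
; SetWeaponState toggles collision and physics for Dropped, Equipped and In Hand, offsetting the mesh by its Handle socket when held.
; The construction script records the actor's own class in WeaponStruct.
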(event `/Game/Blueprints/InteractInterface.Interact`
  (params (Interactor :type "Actor Object Reference"))
  (`/Game/Blueprints/Weapon/WeaponSystemComponent.PickUpWeapon` (`self.GetComponentByClass` Interactor "/Game/Blueprints/Weapon/WeaponSystemComponent.WeaponSystemComponent_C") self))

(event `self.InteractionArea.OnComponentBeginOverlap`
  (params (OverlappedComponent :type "PrimitiveComponent Object Reference") (OtherActor :type "Actor Object Reference") (OtherComp :type "PrimitiveComponent Object Reference") (OtherBodyIndex :type Integer) (bFromSweep :type Boolean) (SweepResult :type "HitResult Structure (by ref)"))
  (bind _widget (`self.Widget`))
  (cast `/Game/Blueprints/Character/BP_PLayerCharacter` OtherActor)
  (set `self.CanPick` true)
  (`self.InteractUI`
    (:`then`
      _)
    (:`else`
      (bind _returnvalue (`|CreateWidget` "/Game/UI/Weapon/InteractWB.InteractWB_C" null (`.WeaponName_4_2B5979084C41D8C9E93C79B682A93349` (break `/Game/Blueprints/Weapon/WeaponStruct` (`self.WeaponStruct`)))))
      (set `self.InteractUI` _returnvalue)
      (`WidgetComponent.SetWidget` _widget _returnvalue)))
  (`SceneComponent.SetVisibility` _widget true false))

(event `self.InteractionArea.OnComponentEndOverlap`
  (params (OverlappedComponent :type "PrimitiveComponent Object Reference") (OtherActor :type "Actor Object Reference") (OtherComp :type "PrimitiveComponent Object Reference") (OtherBodyIndex :type Integer))
  (`SceneComponent.SetVisibility` (`self.Widget`) false false)
  (set `self.CanPick` false))

(fn `SetWeaponState`
  (params (WeaponState :type "/Game/Blueprints/Weapon/WeaponStateEnum Enum" :default "NewEnumerator0"))
  (bind _weaponmesh (`self.WeaponMesh`))
  (bind _weaponmesh_2 (`self.WeaponMesh`))
  (bind _returnvalue_location (`KismetMathLibrary.BreakTransform` (`SceneComponent.GetSocketTransform` _weaponmesh_2 "Handle" "RTS_Component")))
  (switch `/Game/Blueprints/Weapon/WeaponStateEnum` WeaponState
    (:`NewEnumerator0`
      (`PrimitiveComponent.SetCollisionProfileName` (`self.InteractionArea`) "OverlapAllDynamic" false)
      (`PrimitiveComponent.SetCollisionProfileName` (`self.WeaponMesh`) "DroppedGun" false)
      (`PrimitiveComponent.SetSimulatePhysics` (`self.WeaponMesh`) true))
    (:`NewEnumerator1`
      (`PrimitiveComponent.SetCollisionProfileName` (`self.InteractionArea`) "NoCollision" false)
      (`PrimitiveComponent.SetCollisionProfileName` (`self.WeaponMesh`) "NoCollision" false)
      (`PrimitiveComponent.SetSimulatePhysics` _weaponmesh false)
      (`SceneComponent.ResetRelativeTransform` _weaponmesh))
    (:`NewEnumerator2`
      (`PrimitiveComponent.SetCollisionProfileName` (`self.InteractionArea`) "NoCollision" false)
      (`PrimitiveComponent.SetCollisionProfileName` (`self.WeaponMesh`) "NoCollision" false)
      (`PrimitiveComponent.SetSimulatePhysics` (`self.WeaponMesh`) false)
      (`SceneComponent.K2_SetRelativeLocation` _weaponmesh_2 (* _returnvalue_location -1.0) false false))))

(fn `UserConstructionScript`
  (bind (_weaponstruct_weaponname _weaponstruct_weaponenum _weaponstruct_weaponclass _weaponstruct_magsize _weaponstruct_currentammo _weaponstruct_damage _weaponstruct_weaponimage _weaponstruct_ismeleeweapon) (break `/Game/Blueprints/Weapon/WeaponStruct` (`self.WeaponStruct`)))
  (setmembers `/Game/Blueprints/Weapon/WeaponStruct` :`StructRef` (`self.WeaponStruct`) :`WeaponName` _weaponstruct_weaponname :`WeaponEnum` _weaponstruct_weaponenum :`WeaponClass` (`GameplayStatics.GetObjectClass` self) :`MagSize` _weaponstruct_magsize :`CurrentAmmo` _weaponstruct_currentammo :`Damage` _weaponstruct_damage :`WeaponImage` _weaponstruct_weaponimage :`IsMeleeWeapon` _weaponstruct_ismeleeweapon))